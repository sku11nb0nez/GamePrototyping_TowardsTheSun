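; Player-controlled 2D Paper character that moves along the X axis with jump, sneak and sprite flipping, and creates the HUD.
; Jump and landing play sounds and set the animation Blueprint's jump state; Scuttlers entering EnemyDetection get a delayed health update.
; Damage reduces lives on the HUD, pausing into game over at zero.
; Attack animation and stamina-gated jumping logic are disconnected and never run.
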(event `EnhancedInput|/Game/Resources/Character/Inputs/IA_PaperAtttack`
  (params (ActionValue :type Boolean) (ElapsedSeconds :type "Float (double-precision)") (TriggeredSeconds :type "Float (double-precision)") (InputAction :type "InputAction Object Reference" :default "/Game/Resources/Character/Inputs/IA_PaperAtttack.IA_PaperAtttack"))
  ; Player Attack (Unused)
)

(event `self.ReceiveBeginPlay`
  ; Player Movement Mapping Context
  (`EnhancedInputSubsystemInterface.AddMappingContext` (pcsubsystem `EnhancedInputLocalPlayerSubsystem` (`GameplayStatics.GetPlayerController` 0)) "/Game/Resources/Character/Inputs/IMC_PaperPlayer.IMC_PaperPlayer" 0 (struct))
  ; Animation Blueprint Cast
  (bind _asabp_paper_character (cast `/Game/Resources/Character/ABP_PaperCharacter` (`PaperZDAnimationComponent.AnimInstance` (`self.AnimationComponent`))))
  (set `self.Animation BP` _asabp_paper_character)
  ; Adding HUD Widget to Viewport
  (bind _returnvalue (`|CreateWidget` "/Game/Resources/HUD/WB_HUD.WB_HUD_C"))
  (bind _output_get (set `self.HUD` _returnvalue))
  (`UserWidget.AddToViewport` _output_get 0))

(event `EnhancedInput|/Game/Resources/Character/Inputs/IA_PaperJump`
  (params (ActionValue :type "Float (double-precision)") (ElapsedSeconds :type "Float (double-precision)") (TriggeredSeconds :type "Float (double-precision)") (InputAction :type "InputAction Object Reference" :default "/Game/Resources/Character/Inputs/IA_PaperJump.IA_PaperJump"))
  ; Player Jump  and Double Jump
  (:`Triggered`
    (`self.Jump`)
    (set `/Game/Resources/Character/ABP_PaperCharacter.Jumping` true (`self.Animation BP`))
    (`GameplayStatics.PlaySound2D` "/Game/Resources/Sound/Player_Movement/30_Jump_03.30_Jump_03" 1.0 1.0 0.0 null null))
  (:`Completed`
    (`self.StopJumping`)
    (set `CharacterMovementComponent.bNotifyApex` false (`self.CharacterMovement`))))

(event `self.OnLanded`
  (params (Hit :type "HitResult Structure (by ref)"))
  ; Jump Landing
  (set `/Game/Resources/Character/ABP_PaperCharacter.Jumping` false (`self.Animation BP`))
  (`GameplayStatics.PlaySound2D` "/Game/Resources/Sound/Player_Movement/45_Landing_01.45_Landing_01" 1.0 1.0 0.0 null null))

(event `self.ReceiveTick`
  (params (DeltaSeconds :type "Float (single-precision)"))
  ; Gradual Stamina Increase
)

(event `EnhancedInput|/Game/Resources/Character/Inputs/IA_PaperMove`
  (params (ActionValue :type "Float (double-precision)") (ElapsedSeconds :type "Float (double-precision)") (TriggeredSeconds :type "Float (double-precision)") (InputAction :type "InputAction Object Reference" :default "/Game/Resources/Character/Inputs/IA_PaperMove.IA_PaperMove"))
  (bind _returnvalue_x (`KismetMathLibrary.BreakVector` (`self.GetVelocity`)))
  ; Player Move
  (:`Triggered`
    (`self.AddMovementInput` (1.0 0.0 0.0) ActionValue)
    ; Change Direction
    (if (< _returnvalue_x 0.0)
      (`SceneComponent.SetRelativeScale3D` (`self.Sprite`) (1.0 1.0 1.0))
      (else
        (`SceneComponent.SetRelativeScale3D` (`self.Sprite`) (-1.0 1.0 1.0))))))

(event `Key|LeftShift`
  (params (Key :type "Key Structure"))
  ; Player Sneak
  (:`Pressed`
    (set `CharacterMovementComponent.MaxWalkSpeed` 100.0 (`self.CharacterMovement`)))
  (:`Released`
    (set `CharacterMovementComponent.MaxWalkSpeed` 300.0 (`self.CharacterMovement`))))

(event `self.EnemyDetection.OnComponentBeginOverlap`
  (params (OverlappedComponent :type "PrimitiveComponent Object Reference") (OtherActor :type "Actor Object Reference") (OtherComp :type "PrimitiveComponent Object Reference") (OtherBodyIndex :type Integer) (bFromSweep :type Boolean) (SweepResult :type "HitResult Structure (by ref)"))
  ; Player Attack 2
  (bind _asbp_scuttler (cast `/Game/Resources/Enemies/Scuttler/BP_Scuttler` OtherActor))
  (`KismetSystemLibrary.Delay` 0.3)
  (`/Game/Resources/Enemies/Scuttler/BP_Scuttler.UpdateHealth` _asbp_scuttler (`self.DamageTaken`)))

(fn `DeathOperations`
  (bind _returnvalue (`GameplayStatics.GetPlayerController` 0))
  (`GameplayStatics.SetGamePaused` true)
  (set `PlayerController.bShowMouseCursor` true _returnvalue)
  (`WidgetBlueprintLibrary.SetInputMode_UIOnlyEx` _returnvalue null))

(fn `HealthBoost`
  (params (LivesToAdd :type Integer))
  (if (< (`self.Lives`) 5)
    (set `self.Lives` (+ (`self.Lives`) LivesToAdd))
    (`/Game/Resources/HUD/WB_HUD.UpdateLives` (`self.HUD`) 5)))

(fn `HitCheckScuttler`
  (for _array_element (`PrimitiveComponent.GetOverlappingActors` (`self.HitBox`) "/Game/Resources/Enemies/Scuttler/BP_Scuttler.BP_Scuttler_C")
    (if (!= _array_element self)
      (`GameplayStatics.ApplyDamage` _array_element (`self.DamageAmount`)))))

(fn `StaminaBoost`
  (params (StaminaToAdd :type Integer))
  (if (<= (`self.Stamina`) 100)
    (bind _output_get (set `self.Stamina` (+ (`self.Stamina`) StaminaToAdd)))
    (`/Game/Resources/HUD/WB_HUD.UpdateStamina` (`self.HUD`) (`KismetMathLibrary.Clamp` _output_get 0 100))))

(fn `TakeDamage`
  (params (Damage :type Integer))
  (`GameplayStatics.PlaySound2D` "/Game/Resources/Sound/Player_Movement/61_Hit_03.61_Hit_03" 1.0 1.0 0.0 null null)
  (bind _output_get (set `self.Lives` (- (`self.Lives`) Damage)))
  (`/Game/Resources/HUD/WB_HUD.UpdateLives` (`self.HUD`) _output_get)
  (if (== _output_get 0)
    (`Widget.SetVisibility` (`/Game/Resources/HUD/WB_HUD.GameOverScreen` (`self.HUD`)) "Visible")
    (`self.DeathOperations`)
    (`GameplayStatics.PlaySound2D` "/Game/Resources/Sound/BG_Music/Game_Over.Game_Over" 1.0 1.0 0.0 null null)))

(fn `TurnAround`
  ; Player flip when changing walking direction
  (`self.K2_SetActorRotation` (`KismetMathLibrary.ComposeRotators` (`self.K2_GetActorRotation`) (struct :`Yaw` 180.0))))

(fn `UpdateStamina`
  (params (StaminaUsed :type Integer))
  (bind _output_get (set `self.Stamina` (- (`self.Stamina`) StaminaUsed)))
  (`/Game/Resources/HUD/WB_HUD.UpdateStamina` (`self.HUD`) (`KismetMathLibrary.Clamp` _output_get 0 100)))

(fn `UserConstructionScript`)