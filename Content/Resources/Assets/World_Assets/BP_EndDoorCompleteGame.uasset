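; BP_EndDoorCompleteGame is the level's end door, which completes the game when the paper character overlaps it holding exactly the required coin count.
; On a match it shows the HUD's game complete screen, pauses the game, switches to UI-only input with the cursor visible and plays a victory sound.
; Any other coin count plays a denied sound instead.
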(event `self.ReceiveActorBeginOverlap`
  (params (OtherActor :type "Actor Object Reference"))
  (bind _returnvalue (`GameplayStatics.GetPlayerController` 0))
  (bind _asbp_paper_character (cast `/Game/Resources/Character/BP_PaperCharacter` OtherActor))
  (if (== (`/Game/Resources/Character/BP_PaperCharacter.Coins` _asbp_paper_character) (`self.CoinsNeeded`))
    ; Open Game Complete Screen
    (set `self.As BP Paper Character` _asbp_paper_character)
    (`Widget.SetVisibility` (`/Game/Resources/HUD/WB_HUD.GameCompleteScreen` (`/Game/Resources/Character/BP_PaperCharacter.HUD` (`self.As BP Paper Character`))) "Visible")
    (set `PlayerController.bShowMouseCursor` true _returnvalue)
    (`GameplayStatics.SetGamePaused` true)
    (`WidgetBlueprintLibrary.SetInputMode_UIOnlyEx` _returnvalue null)
    (`GameplayStatics.PlaySound2D` "/Game/Resources/Sound/BG_Music/Victory.Victory" 1.0 1.0 0.0 null null)
    (else
      (`GameplayStatics.PlaySound2D` "/Game/Resources/Sound/UI_Sound_Effects/033_Denied_03.033_Denied_03" 1.0 1.0 0.0 null null))))

(fn `UserConstructionScript`)