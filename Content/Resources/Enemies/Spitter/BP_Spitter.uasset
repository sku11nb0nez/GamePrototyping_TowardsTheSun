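; BP_Spitter is a patrolling enemy that walks forward every tick and damages BP_PaperCharacter on contact.
; Wall overlap begin and ledge overlap end both call TurnAround, which rotates the actor 180 degrees to reverse the patrol.
; Touching the player also turns it around, with a DoOnce and short delay limiting repeated turns but not the damage.
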(event `self.ReceiveTick`
  (params (DeltaSeconds :type "Float (single-precision)"))
  (`self.AddMovementInput` (`self.GetActorForwardVector`)))

(event `self.PlayerDetection.OnComponentBeginOverlap`
  (params (OverlappedComponent :type "PrimitiveComponent Object Reference") (OtherActor :type "Actor Object Reference") (OtherComp :type "PrimitiveComponent Object Reference") (OtherBodyIndex :type Integer) (bFromSweep :type Boolean) (SweepResult :type "HitResult Structure (by ref)"))
  ; Enemy Player Detection
  (bind _asbp_paper_character (cast `/Game/Resources/Character/BP_PaperCharacter` OtherActor))
  (`/Game/Resources/Character/BP_PaperCharacter.TakeDamage` _asbp_paper_character (`self.DamageAmount`))
  (`/Engine/EditorBlueprintResources/StandardMacros.DoOnce` false :!label _label
    (:`Completed`
      (`self.TurnAround`)
      (`KismetSystemLibrary.Delay` 0.2)
      (goto _label :!via `Reset`))))

(event `self.WallDetection.OnComponentBeginOverlap`
  (params (OverlappedComponent :type "PrimitiveComponent Object Reference") (OtherActor :type "Actor Object Reference") (OtherComp :type "PrimitiveComponent Object Reference") (OtherBodyIndex :type Integer) (bFromSweep :type Boolean) (SweepResult :type "HitResult Structure (by ref)"))
  ; Enemy Wall and Ledge Detection Turn Around
  (`self.TurnAround` :!label _label_2))

(event `self.LedgeDetection.OnComponentEndOverlap`
  (params (OverlappedComponent :type "PrimitiveComponent Object Reference") (OtherActor :type "Actor Object Reference") (OtherComp :type "PrimitiveComponent Object Reference") (OtherBodyIndex :type Integer))
  ; Enemy Wall and Ledge Detection Turn Around
  (goto _label_2))

(fn `TurnAround`
  (`self.K2_SetActorRotation` (`KismetMathLibrary.ComposeRotators` (`self.K2_GetActorRotation`) (struct :`Yaw` 180.0))))

(fn `UserConstructionScript`)