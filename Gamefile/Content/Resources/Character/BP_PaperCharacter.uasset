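; BP_PaperCharacter is a player-controlled Paper character that runs along the world X axis and jumps.
; BeginPlay registers the IMC_PaperPlayer Enhanced Input context and caches the ABP_PaperCharacter instance from its AnimationComponent.
; The move action feeds movement input along X only.
; Jump input triggers the jump and sets the animation blueprint's Jumping flag, which OnLanded clears.
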(event `self.ReceiveBeginPlay`
  ; Player Movement Mapping Context
  (`EnhancedInputSubsystemInterface.AddMappingContext` (pcsubsystem `EnhancedInputLocalPlayerSubsystem` (`GameplayStatics.GetPlayerController` 0)) "/Game/Resources/Character/Inputs/IMC_PaperPlayer.IMC_PaperPlayer" 0 (struct))
  ; Animation Blueprint Cast
  (bind _asabp_paper_character (cast `/Game/Resources/Character/ABP_PaperCharacter` (`PaperZDAnimationComponent.AnimInstance` (`self.AnimationComponent`))))
  (set `self.Animation BP` _asabp_paper_character))

(event `EnhancedInput|/Game/Resources/Character/Inputs/IA_PaperJump`
  (params (ActionValue :type Boolean) (ElapsedSeconds :type "Float (double-precision)") (TriggeredSeconds :type "Float (double-precision)") (InputAction :type "InputAction Object Reference" :default "/Game/Resources/Character/Inputs/IA_PaperJump.IA_PaperJump"))
  ; Player Jump
  (:`Started`
    (`self.Jump`)
    (set `/Game/Resources/Character/ABP_PaperCharacter.Jumping` true (`self.Animation BP`)))
  (:`Completed`
    (`self.StopJumping`)))

(event `self.OnLanded`
  (params (Hit :type "HitResult Structure (by ref)"))
  ; Player Jump
  (set `/Game/Resources/Character/ABP_PaperCharacter.Jumping` false (`self.Animation BP`)))

(event `EnhancedInput|/Game/Resources/Character/Inputs/IA_PaperMove`
  (params (ActionValue :type "Float (double-precision)") (ElapsedSeconds :type "Float (double-precision)") (TriggeredSeconds :type "Float (double-precision)") (InputAction :type "InputAction Object Reference" :default "/Game/Resources/Character/Inputs/IA_PaperMove.IA_PaperMove"))
  ; Player Move
  (:`Triggered`
    (`self.AddMovementInput` (1.0 0.0 0.0) ActionValue)))

(fn `UserConstructionScript`)