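; BP_Scuttler is a patrolling enemy that constantly walks forward and damages the player character on contact.
; Overlap components drive it: touching a wall, losing ledge overlap or hitting the player flips it 180 degrees, with a DoOnce and short delay throttling player-triggered turns.
; UpdateHealth handles death with sound and destruction, but nothing here calls it; received damage is only printed.
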(event `self.ReceiveTick`
  (params (DeltaSeconds :type "Float (single-precision)"))
  ; Enemy Movement
  (`self.AddMovementInput` (`self.GetActorForwardVector`)))

(event `self.PlayerDetection.OnComponentBeginOverlap`
  (params (OverlappedComponent :type "PrimitiveComponent Object Reference") (OtherActor :type "Actor Object Reference") (OtherComp :type "PrimitiveComponent Object Reference") (OtherBodyIndex :type Integer) (bFromSweep :type Boolean) (SweepResult :type "HitResult Structure (by ref)"))
  ; Enemy Player Detection
  (bind _asbp_paper_character (cast `/Game/Resources/Character/BP_PaperCharacter` OtherActor))
  (`/Game/Resources/Character/BP_PaperCharacter.TakeDamage` _asbp_paper_character (`self.DamageAmount`))
  (`/Engine/EditorBlueprintResources/StandardMacros.DoOnce` false :!label _label
    (:`Completed`
      (`self.TurnAround`)
      (`KismetSystemLibrary.Delay` 0.2)
      (goto _label :!via `Reset`))))

(event `self.WallDetection.OnComponentBeginOverlap`
  (params (OverlappedComponent :type "PrimitiveComponent Object Reference") (OtherActor :type "Actor Object Reference") (OtherComp :type "PrimitiveComponent Object Reference") (OtherBodyIndex :type Integer) (bFromSweep :type Boolean) (SweepResult :type "HitResult Structure (by ref)"))
  ; Wall and Ledge Detection Turn Around
  (`self.TurnAround` :!label _label_2))

(event `self.ReceiveAnyDamage`
  (params (Damage :type "Float (single-precision)") (DamageType :type "DamageType Object Reference") (InstigatedBy :type "Controller Object Reference") (DamageCauser :type "Actor Object Reference"))
  (`KismetSystemLibrary.PrintString` (`KismetStringLibrary.Concat_StrStr` "Taken Damage" (`KismetStringLibrary.Conv_DoubleToString` Damage))))

(event `self.LedgeDetection.OnComponentEndOverlap`
  (params (OverlappedComponent :type "PrimitiveComponent Object Reference") (OtherActor :type "Actor Object Reference") (OtherComp :type "PrimitiveComponent Object Reference") (OtherBodyIndex :type Integer))
  ; Wall and Ledge Detection Turn Around
  (goto _label_2))

(fn `TurnAround`
  (`self.K2_SetActorRotation` (`KismetMathLibrary.ComposeRotators` (`self.K2_GetActorRotation`) (struct :`Yaw` 180.0))))

(fn `UpdateHealth`
  (params (Damage :type Integer))
  (bind _output_get (set `self.Health` (- (`self.Health`) Damage)))
  (if (<= _output_get 0)
    (`GameplayStatics.PlaySound2D` "/Game/Resources/Sound/Combat_Sounds/69_Enemy_death_01.69_Enemy_death_01" 1.0 1.0 0.0 null null)
    (`self.K2_DestroyActor`)))

(fn `UserConstructionScript`)